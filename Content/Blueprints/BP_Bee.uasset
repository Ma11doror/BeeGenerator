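; BP_Bee is a modular bee whose body, wings, legs and antenna are separate skeletal mesh components.
; Legs, wings and antenna follow the body Mesh as leader pose, set in both the construction script and BeginPlay.
; ApplyBodyPart takes a body part asset and swaps its skeletal mesh into the slot matching its part type, skipping invalid meshes.
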(event `self.ReceiveBeginPlay`
  (`self.SetupMasterPose`))

(event `self.ApplyBodyPart`
  (params (InBodyPartAsset :type "BodyPartAsset Object Reference"))
  (bind _bodypartskeletalmesh (`BodyPartAsset.BodyPartSkeletalMesh` InBodyPartAsset)
    (:`then`
      (`SkeletalMeshComponent.SetSkeletalMeshAsset` (select `EBodyPartType` (`BodyPartAsset.BodyPartType` InBodyPartAsset) :`Body` (`self.Mesh`) :`Wings` (`self.WingsSlot`) :`Legs` (`self.LegsSlot`) :`Antenna` (`self.AntennaSlot`)) _bodypartskeletalmesh))
    (:`else`)))

(fn `SetupMasterPose`
  (`SkinnedMeshComponent.SetLeaderPoseComponent` (`self.LegsSlot`) (`self.Mesh`) false false)
  (`SkinnedMeshComponent.SetLeaderPoseComponent` (`self.WingsSlot`) (`self.Mesh`) false false)
  (`SkinnedMeshComponent.SetLeaderPoseComponent` (`self.AntennaSlot`) (`self.Mesh`) false false))

(fn `UserConstructionScript`
  (`self.SetupMasterPose`))